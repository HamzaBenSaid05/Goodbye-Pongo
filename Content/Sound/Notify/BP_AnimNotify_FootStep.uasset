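; Anim notify that plays surface-dependent footstep sounds for TPP_CharacterBase characters.
; On notify, it line-traces downward from the owning character and reads the hit physical material's surface type.
; It then plays the footstep tag through the character's sound component, passing a Material integer parameter to distinguish Grass, Stone and the default surface.
; Owners that are not TPP_CharacterBase only print a debug message.
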(fn `Received_Notify`
  (params (MeshComp :type "SkeletalMeshComponent Object Reference") (Animation :type "AnimSequenceBase Object Reference") (EventReference :type "AnimNotifyEventReference Structure (by ref)"))
  (returns (ReturnValue :type Boolean))
  (locals (Character :type "TPP_CharacterBase Object Reference") (SoundComponent :type "TPP_SoundComponent Object Reference"))
  (bind _character (`local.Character`))
  (bind _character_2 (`local.Character`))
  (bind _character_3 (`local.Character`))
  (bind _astpp_character_base (cast `TPP_CharacterBase` (`ActorComponent.GetOwner` MeshComp))
    (:`then`
      (bind _output_get (set `local.Character` _astpp_character_base))
      (bind _returnvalue (`Actor.K2_GetActorLocation` _astpp_character_base))
      (bind (_outhit _returnvalue_2) (`KismetSystemLibrary.LineTraceSingle` _returnvalue (- _returnvalue (0.0 0.0 300.0)) "TraceTypeQuery1" false (`|MakeArray` _output_get :!type "Actor Object Reference")))
      (if _returnvalue_2
        (bind _returnvalue_3 (`TPP_CharacterBase.GetSoundComponent` (`local.Character`)))
        (set `local.SoundComponent` _returnvalue_3)
        (switch `EPhysicalSurface` (`PhysicalMaterial.SurfaceType` (`.PhysMat` (`GameplayStatics.BreakHitResult` _outhit)))
          (:`SurfaceType_Default`
            (`TPP_SoundComponent.PlaySound` (`local.SoundComponent`) (`self.TagFootstep`) (`Actor.K2_GetActorLocation` _character_2) (make `TPP_AudioParameter` 0 "Material") (`Actor.RootComponent` _character_2)))
          (:`SurfaceType1`
            (`TPP_SoundComponent.PlaySound` (`local.SoundComponent`) (`self.TagFootstep`) (`Actor.K2_GetActorLocation` _character) (make `TPP_AudioParameter` 1 "Material") (`Actor.RootComponent` _character)))
          (:`SurfaceType2`
            (`TPP_SoundComponent.PlaySound` (`local.SoundComponent`) (`self.TagFootstep`) (`Actor.K2_GetActorLocation` _character_3) (make `TPP_AudioParameter` 2 "Material") (`Actor.RootComponent` _character_3))))
        (return true)))
    (:`CastFailed`
      (`KismetSystemLibrary.PrintText` "Non sono un character Base")
      (return false))))
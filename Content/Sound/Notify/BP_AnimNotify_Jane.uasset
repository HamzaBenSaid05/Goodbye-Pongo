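; Animation notify (Jane) that triggers a tagged sound on a third-person character during an animation.
; It casts the mesh owner to TPP_CharacterBase and does nothing further if the cast fails.
; It then calls PlaySound on the character's sound component with the notify's Tag, the actor location, the root component as source, and an integer passed as the "Action" parameter.
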(fn `Received_Notify`
  (params (MeshComp :type "SkeletalMeshComponent Object Reference") (Animation :type "AnimSequenceBase Object Reference") (EventReference :type "AnimNotifyEventReference Structure (by ref)"))
  (returns (ReturnValue :type Boolean))
  (locals (Character :type "TPP_CharacterBase Object Reference") (SoundComponent :type "TPP_SoundComponent Object Reference"))
  (bind _character (`local.Character`))
  (bind _astpp_character_base (cast `TPP_CharacterBase` (`ActorComponent.GetOwner` MeshComp)))
  (set `local.Character` _astpp_character_base)
  (bind _returnvalue (`TPP_CharacterBase.GetSoundComponent` (`local.Character`)))
  (set `local.SoundComponent` _returnvalue)
  (`TPP_SoundComponent.PlaySound` (`local.SoundComponent`) (`self.Tag`) (`Actor.K2_GetActorLocation` _character) (make `TPP_AudioParameter` (`self.Parameter Int`) "Action") (`Actor.RootComponent` _character))
  (return true))
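; Player controller that adds the UI input mapping context and caches Pongo's AI controller from either the main or test game mode.
; It tracks whether the last key pressed came from a gamepad.
; HandleOptionMenu pushes the option menu onto the HUD's menu layer and pauses the game.
; Disconnected debug logic remains for teleporting, save reset, level reload, time dilation and toggling Pongo's fear and stroll states.
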(event `self.ReceiveBeginPlay`
  (bind _returnvalue (`GameplayStatics.GetGameMode`))
  (`parent.ReceiveBeginPlay`)
  (message `EnhancedInputSubsystemInterface.AddMappingContext` (pcsubsystem `EnhancedInputLocalPlayerSubsystem` self) "/Game/Input/IMC_UI.IMC_UI" 0 (struct))
  (bind _asbp_main_game_mode (cast `/Game/Blueprints/Gameplay/GameModes/BP_MainGameMode` _returnvalue)
    (:`then`
      (bind _returnvalue_2 (`TPP_GameMode.GetPongoRef` _asbp_main_game_mode))
      (`/Engine/EditorBlueprintResources/StandardMacros.IsValid` _returnvalue_2
        (:`Is Valid`
          (bind _astpp_pongo_controller (cast `TPP_PongoController` (`Pawn.GetController` _returnvalue_2)))
          (set `self.AIController` _astpp_pongo_controller))))
    (:`CastFailed`
      (bind _asbp_test_game_mode (cast `/Game/Blueprints/Gameplay/GameModes/BP_TestGameMode` _returnvalue))
      (bind _returnvalue_3 (`TPP_TestingGameMode.GetPongoRef` _asbp_test_game_mode))
      (`/Engine/EditorBlueprintResources/StandardMacros.IsValid` _returnvalue_3
        (:`Is Valid`
          (bind _astpp_pongo_controller_2 (cast `TPP_PongoController` (`Pawn.GetController` _returnvalue_3)))
          (set `self.AIController` _astpp_pongo_controller_2))))))

(event `Key|AnyKey` :consume false
  (params (Key :type "Key Structure"))
  (:`Pressed`
    (bind _output_get (set `self.LastInputKey` Key))
    (set `self.bIsController` (`KismetInputLibrary.Key_IsGamepadKey` _output_get))))

(event `Key|F3`
  (params (Key :type "Key Structure")))

(event `self.HandleOptionMenu`
  (bind _astpp_hud (cast `TPP_HUD` (`self.GetHUD`)))
  (`TPP_HUD.PushWidgetToLayer` _astpp_hud (struct :`TagName` "UI.Layer.Menu") "/Game/Blueprints/UI/OptionMenu/WBP_OptionMenu.WBP_OptionMenu_C")
  (`GameplayStatics.SetGamePaused` true))

(event `Key|F4`
  (params (Key :type "Key Structure"))
  ;[1 0.6501 0 0.5] Save & Reload
)

(event `Key|N`
  (params (Key :type "Key Structure"))
  ;[0.4635 0 0 0.5] PongoState Fear From Player
)

(event `Key|M`
  (params (Key :type "Key Structure"))
  ;[0.4635 0 0 0.5] PongoState Stroll
)

(event `Key|Shift+F4`
  (params (Key :type "Key Structure"))
  ;[1 0.6501 0 0.5] Save & Reload
)

(event `Key|Tab`
  (params (Key :type "Key Structure"))
  ;[0 1 0.1349 0.5] Slomo
)

(event `Key|Shift+Tab`
  (params (Key :type "Key Structure"))
  ;[0 1 0.1349 0.5] Slomo
)

(fn `UserConstructionScript`)
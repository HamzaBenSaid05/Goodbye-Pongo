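; Final-scene trigger actor that times scripted reactions to a camera zoom on the Huk Runa head.
; It binds to the camera's zoom component and, on the HukRunaHeadZoomTrigger state, starts timers for the head glow and Pongo's rage color.
; The glow boosts emissive on a dynamic material instance.
; After the color change, another timer leads to tagging Pongo and switching its controller's emotional state to Scripted.
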(event `self.ReceiveBeginPlay`
  (add `TPP_CameraZoomComponent.OnCameraZoom` (`TPP_Camera.CameraZoomComponent` (`self.Camera`)) (`|CreateDelegate` :!event `OnCameraZoom`)))

(fn `ChangePongoColor`
  (bind _pongoref (`/Game/Blueprints/BP_Statics.GetPongoRef` self))
  (message `TPP_AIAction.SetColor` _pongoref (`self.PongoColorRage`))
  (`KismetSystemLibrary.K2_SetTimerDelegate` (`|CreateDelegate` :!event `SetPongoScritped`) (`self.TimerPongoScriptedEventAfterColorChanging`)))

(fn `LightUpHukRunaHead`
  (bind _returnvalue (`PrimitiveComponent.CreateDynamicMaterialInstance` (`StaticMeshActor.StaticMeshComponent` (`self.HukRunaHead`)) 0 "/Game/Art/Materials/HukRuna/MI_HukRunaHead.MI_HukRunaHead" "None"))
  (`MaterialInstanceDynamic.SetScalarParameterValue` _returnvalue (`self.EmissiveBoostParameterName`) 50.0))

(fn `OnCameraZoom`
  (params (State :type "EZoomTrigger Enum" :default "OnZoomInStart"))
  (if (`|EnumEquality` State (`self.HukRunaHeadZoomTrigger`))
    (`KismetSystemLibrary.K2_SetTimerDelegate` (`|CreateDelegate` :!event `LightUpHukRunaHead`) (`self.TimerHukRuneHeadLightUp`))
    (`KismetSystemLibrary.K2_SetTimerDelegate` (`|CreateDelegate` :!event `ChangePongoColor`) (`self.TimerPongoRageColor`))))

(fn `SetPongoScritped`
  (bind _pongoref (`/Game/Blueprints/BP_Statics.GetPongoRef` self))
  (`TPP_AITaggable.AddGameplayTag` _pongoref (`self.Tag`))
  (`TPP_PongoController.SetEmotionalState` (`TPP_Pongo.GetPongoController` _pongoref) "Scripted" (`self.Emotional State`)))

(fn `UserConstructionScript`
  (`parent.UserConstructionScript`))
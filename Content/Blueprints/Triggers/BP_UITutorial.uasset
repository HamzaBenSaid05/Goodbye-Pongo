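; BP_UITutorial is a tutorial trigger actor that shows or hides a world UI hint through its WidgetComponent.
; TriggerTutorial makes the component visible and calls PlayAnimationB on its WBP_BaseTutorialWidget.
; TriggerTutorialOut hides the component and then calls PlayAnimationF on the same widget.
; It has no overlap, tick or construction logic of its own, so both events rely on outside callers.
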(event `self.TriggerTutorial`
  (bind _widgetcomponent (`self.WidgetComponent`))
  (`SceneComponent.SetVisibility` _widgetcomponent true false)
  (bind _aswbp_base_tutorial_widget (cast `/Game/Blueprints/UI/TestInteractUi/WBP_BaseTutorialWidget` (`WidgetComponent.GetWidget` _widgetcomponent)))
  (`/Game/Blueprints/UI/TestInteractUi/WBP_BaseTutorialWidget.PlayAnimationB` _aswbp_base_tutorial_widget))

(event `self.TriggerTutorialOut`
  (bind _widgetcomponent (`self.WidgetComponent`))
  (`SceneComponent.SetVisibility` _widgetcomponent false false)
  (bind _aswbp_base_tutorial_widget (cast `/Game/Blueprints/UI/TestInteractUi/WBP_BaseTutorialWidget` (`WidgetComponent.GetWidget` _widgetcomponent)))
  (`/Game/Blueprints/UI/TestInteractUi/WBP_BaseTutorialWidget.PlayAnimationF` _aswbp_base_tutorial_widget))

(fn `UserConstructionScript`)
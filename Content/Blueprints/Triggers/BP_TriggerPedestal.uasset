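; BP_TriggerPedestal is a trigger volume that shows a widget when the player is near a referenced pedestal that has no orb.
; Box overlaps with the player character turn Tick on when entering, and turn it off and hide the widget when leaving.
; While ticking, it polls the pedestal's Orb reference, showing the widget if the orb is missing and hiding it otherwise.
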(event `self.ReceiveTick`
  (params (DeltaSeconds :type "Float (single-precision)"))
  (bind _pedestalref (`self.PedestalRef`))
  (`/Engine/EditorBlueprintResources/StandardMacros.IsValid` _pedestalref
    (:`Is Valid`
      (`/Engine/EditorBlueprintResources/StandardMacros.IsValid` (`TPP_PedestalItemBase.Orb` _pedestalref)
        (:`Is Valid`
          (`SceneComponent.SetVisibility` (`self.Widget`) false false))
        (:`Is Not Valid`
          (`SceneComponent.SetVisibility` (`self.Widget`) true false))))))

(event `self.Box.OnComponentBeginOverlap`
  (params (OverlappedComponent :type "PrimitiveComponent Object Reference") (OtherActor :type "Actor Object Reference") (OtherComp :type "PrimitiveComponent Object Reference") (OtherBodyIndex :type Integer) (bFromSweep :type Boolean) (SweepResult :type "HitResult Structure (by ref)"))
  (cast `TPP_PlayerCharacter` OtherActor)
  (`self.SetActorTickEnabled` true))

(event `self.Box.OnComponentEndOverlap`
  (params (OverlappedComponent :type "PrimitiveComponent Object Reference") (OtherActor :type "Actor Object Reference") (OtherComp :type "PrimitiveComponent Object Reference") (OtherBodyIndex :type Integer))
  (cast `TPP_PlayerCharacter` OtherActor)
  (`self.SetActorTickEnabled` false)
  (`SceneComponent.SetVisibility` (`self.Widget`) false false))

(fn `UserConstructionScript`)
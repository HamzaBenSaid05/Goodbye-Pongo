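; Actor component that makes its owner fall along Z once TriggerFall is called, apparently for dropping objects that are later destroyed.
; TriggerFall enables ticking and starts a destruction timer.
; Each tick moves the owner with a sweep, either accumulating gravity or using constant velocity, after BeginPlay adjusts positive values, likely negating them to point downward.
; DestroyActor removes directly attached actors, then the owner.
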(event `self.ReceiveBeginPlay`
  (bind _result (`self.CheckValue` (`self.Gravity`)))
  (set `self.Gravity` _result)
  (bind _result_2 (`self.CheckValue` (`self.Velocity`)))
  (set `self.Velocity` _result_2))

(event `self.ReceiveTick`
  (params (DeltaSeconds :type "Float (single-precision)"))
  (if (`self.bIsFalling`)
    (if (`self.bUseGravity`)
      (`self.FallActorWithGravity`)
      (else
        (`self.FallActorWithVelocity`)))))

(fn `CheckValue`
  (params (ValueToCheck :type "Float (double-precision)"))
  (returns (Result :type "Float (double-precision)"))
  (if (> ValueToCheck 0.0)
    (bind _result (`/Engine/EditorBlueprintResources/StandardMacros.NegateFloat` (`local.ValueToCheck`))
      (:`  `
        (return _result)))
    (else
      (return (`local.ValueToCheck`)))))

(fn `DestroyActor`
  (for _array_element (`Actor.GetAttachedActors` (`self.GetOwner`) true false)
    (`Actor.K2_DestroyActor` _array_element))
  (`Actor.K2_DestroyActor` (`self.GetOwner`)))

(fn `FallActorWithGravity`
  (bind (_returnvalue_x _returnvalue_y) (`KismetMathLibrary.BreakVector` (`Actor.K2_GetActorLocation` (`self.GetOwner`))))
  (bind (_returnvalue_x_2 _returnvalue_y_2 _returnvalue_z) (`KismetMathLibrary.BreakVector` (`Actor.K2_GetActorLocation` (`self.GetOwner`))))
  (bind _output_get (set `self.CurrentVelocityZ` (+ (`self.CurrentVelocityZ`) (* (`self.Gravity`) (`GameplayStatics.GetWorldDeltaSeconds`)))))
  (`Actor.K2_SetActorLocation` (`self.GetOwner`) (`KismetMathLibrary.MakeVector` _returnvalue_x _returnvalue_y (+ (* _output_get (`GameplayStatics.GetWorldDeltaSeconds`)) _returnvalue_z)) true false))

(fn `FallActorWithVelocity`
  (bind (_returnvalue_x _returnvalue_y) (`KismetMathLibrary.BreakVector` (`Actor.K2_GetActorLocation` (`self.GetOwner`))))
  (bind (_returnvalue_x_2 _returnvalue_y_2 _returnvalue_z) (`KismetMathLibrary.BreakVector` (`Actor.K2_GetActorLocation` (`self.GetOwner`))))
  (`Actor.K2_SetActorLocation` (`self.GetOwner`) (`KismetMathLibrary.MakeVector` _returnvalue_x _returnvalue_y (+ _returnvalue_z (* (`self.Velocity`) (`GameplayStatics.GetWorldDeltaSeconds`)))) true false))

(fn `TriggerFall`
  (set `self.bIsFalling` true)
  (`self.SetComponentTickEnabled` true)
  (`KismetSystemLibrary.K2_SetTimerDelegate` (`|CreateDelegate` :!event `DestroyActor`) (`self.TimerDestory`)))
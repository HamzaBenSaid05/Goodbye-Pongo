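; Game camera that drives see-through cutouts when geometry blocks its view of the player or companion Pongo.
; BeginPlay sets the companion from the first BP_CharacterBase found.
; Each tick, Trace sphere-traces from near each character to the camera, storing hit points or easing back to character positions.
; UpdateSeeThroughCollection writes those positions and interpolated cutout transitions to MPC_SeeThrough, closing cutouts at half their opening speed.
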(event `self.ReceiveBeginPlay`
  (`parent.ReceiveBeginPlay`)
  (bind _returnvalue (`GameplayStatics.GetActorOfClass` "/Game/Blueprints/Characters/BP_CharacterBase.BP_CharacterBase_C"))
  (`self.SetCompanionRef` _returnvalue))

(event `self.ReceiveTick`
  (params (DeltaSeconds :type "Float (single-precision)"))
  (`parent.ReceiveTick` DeltaSeconds)
  (`self.Trace`)
  (`self.UpdateSeeThroughCollection` DeltaSeconds))

(fn `Trace`
  (locals (PlayerPos :type "Vector Structure") (PongoPos :type "Vector Structure"))
  (bind _playerpos (`local.PlayerPos`))
  (bind _pongopos (`local.PongoPos`))
  (bind _returnvalue (`SceneComponent.K2_GetComponentLocation` (`self.CameraComp`)))
  (bind _returnvalue_2 (`SceneComponent.K2_GetComponentLocation` (`self.CameraComp`)))
  (`|ExecutionSequence`
    (:`then_0`
      (bind _playerref (`self.PlayerRef`)
        (:`then`
          (set `local.PlayerPos` (`self.K2_GetActorLocation` _playerref))
          (bind (_outhit _returnvalue_3) (`KismetSystemLibrary.SphereTraceSingle` :`Start` (- _playerpos (* (`KismetMathLibrary.Normal` (- _playerpos _returnvalue)) 50.0)) :`End` _returnvalue :`Radius` 50.0 :`TraceChannel` "TraceTypeQuery1" :`DrawTime` 0.05))
          (bind _output_get (set `self.IsPlayerOccluded` _returnvalue_3))
          (if _output_get
            (set `self.AdjustedPlayerEndTracePos` (`.ImpactPoint` (`GameplayStatics.BreakHitResult` _outhit)))
            (else
              (set `self.AdjustedPlayerEndTracePos` (`KismetMathLibrary.VInterpTo` (`self.AdjustedPlayerEndTracePos`) (`local.PlayerPos`) (`GameplayStatics.GetWorldDeltaSeconds`) 2.0)))))
        (:`else`)))
    (:`then_1`
      (bind _companionref (`self.CompanionRef`)
        (:`then`
          (set `local.PongoPos` (`self.K2_GetActorLocation` _companionref))
          (bind (_outhit_2 _returnvalue_4) (`KismetSystemLibrary.SphereTraceSingle` :`Start` (- _pongopos (* (`KismetMathLibrary.Normal` (- _pongopos _returnvalue_2)) 50.0)) :`End` _returnvalue_2 :`Radius` 50.0 :`TraceChannel` "TraceTypeQuery1" :`DrawTime` 0.5))
          (bind _output_get_2 (set `self.IsPongoOccluded` _returnvalue_4))
          (if _output_get_2
            (set `self.AdjustedPongoEndTracePos` (`.ImpactPoint` (`GameplayStatics.BreakHitResult` _outhit_2)))
            (else
              (set `self.AdjustedPongoEndTracePos` (`KismetMathLibrary.VInterpTo` (`self.AdjustedPongoEndTracePos`) (`local.PongoPos`) (`GameplayStatics.GetWorldDeltaSeconds`) 2.0)))))
        (:`else`)))))

(fn `UpdateSeeThroughCollection`
  (params (DeltaTime :type "Float (double-precision)"))
  (bind _returnvalue (`KismetMathLibrary.FInterpTo` (`self.CurrentPlayerCutout`) 1.0 (`local.DeltaTime`) (`self.CutoutSpeed`)))
  (bind _returnvalue_2 (`KismetMathLibrary.FInterpTo` (`self.CurrentPongoCutout`) 1.0 (`local.DeltaTime`) (`self.CutoutSpeed`)))
  (bind _returnvalue_3 (`KismetMathLibrary.FInterpTo` (`self.CurrentPongoCutout`) 0.0 (`local.DeltaTime`) (* (`self.CutoutSpeed`) 0.5)))
  (bind _returnvalue_4 (`KismetMathLibrary.FInterpTo` (`self.CurrentPlayerCutout`) 0.0 (`local.DeltaTime`) (* (`self.CutoutSpeed`) 0.5)))
  (bind _returnvalue_5 (`KismetMaterialLibrary.GetScalarParameterValue` "/Game/Art/Materials/SeeThrough/MPC_SeeThrough.MPC_SeeThrough" "PlayerCutoutTransition"))
  (set `self.CurrentPlayerCutout` _returnvalue_5)
  (bind _returnvalue_6 (`KismetMaterialLibrary.GetScalarParameterValue` "/Game/Art/Materials/SeeThrough/MPC_SeeThrough.MPC_SeeThrough" "PongoCutoutTransition"))
  (set `self.CurrentPongoCutout` _returnvalue_6)
  (`KismetMaterialLibrary.SetVectorParameterValue` "/Game/Art/Materials/SeeThrough/MPC_SeeThrough.MPC_SeeThrough" "PlayerPos" (`KismetMathLibrary.Conv_VectorToLinearColor` (`self.AdjustedPlayerEndTracePos`)))
  (`KismetMaterialLibrary.SetVectorParameterValue` "/Game/Art/Materials/SeeThrough/MPC_SeeThrough.MPC_SeeThrough" "PongoPos" (`KismetMathLibrary.Conv_VectorToLinearColor` (`self.AdjustedPongoEndTracePos`)))
  (`|ExecutionSequence`
    (:`then_0`
      (if (`self.IsPlayerOccluded`)
        (`KismetMaterialLibrary.SetScalarParameterValue` "/Game/Art/Materials/SeeThrough/MPC_SeeThrough.MPC_SeeThrough" "PlayerCutoutTransition" _returnvalue)
        (set `self.CurrentPlayerCutout` _returnvalue)
        (else
          (`KismetMaterialLibrary.SetScalarParameterValue` "/Game/Art/Materials/SeeThrough/MPC_SeeThrough.MPC_SeeThrough" "PlayerCutoutTransition" _returnvalue_4)
          (set `self.CurrentPlayerCutout` _returnvalue_4))))
    (:`then_1`
      (if (`self.IsPongoOccluded`)
        (`KismetMaterialLibrary.SetScalarParameterValue` "/Game/Art/Materials/SeeThrough/MPC_SeeThrough.MPC_SeeThrough" "PongoCutoutTransition" _returnvalue_2)
        (set `self.CurrentPongoCutout` _returnvalue_2)
        (else
          (`KismetMaterialLibrary.SetScalarParameterValue` "/Game/Art/Materials/SeeThrough/MPC_SeeThrough.MPC_SeeThrough" "PongoCutoutTransition" _returnvalue_3)
          (set `self.CurrentPongoCutout` _returnvalue_3))))))

(fn `UserConstructionScript`)
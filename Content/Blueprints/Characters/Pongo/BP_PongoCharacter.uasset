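; BP_PongoCharacter is the Pongo character, with a collar that can pulse and reaction effects.
; The construction script makes the fur mesh follow the main mesh's pose as leader.
; TogglePulse switches a ColorRatio parameter on a dynamic collar material made at BeginPlay.
; PlayReactionVFX looks up a frame in a reactions data asset, activates the effect and flags it as playing until the system finishes.
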(event `self.ReceiveBeginPlay`
  (bind _mesh (`self.Mesh`))
  (bind _returnvalue (`PrimitiveComponent.CreateDynamicMaterialInstance` _mesh 0 (`PrimitiveComponent.GetMaterial` _mesh 0) "None"))
  (set `self.CollarMI` _returnvalue)
  (add `NiagaraComponent.OnSystemFinished` (`self.ReactionsVFX`) (delegate `SetReactionPlayingBool`)))

(event `SetReactionPlayingBool`
  (params (PSystem :type "NiagaraComponent Object Reference"))
  (set `self.bIsPlayingReactionVFX` false))

(event `self.TogglePulse`
  (params (bTurnOn :type Boolean))
  (`MaterialInstanceDynamic.SetScalarParameterValue` (`self.CollarMI`) "ColorRatio" (`KismetMathLibrary.SelectFloat` 1.0 0.0 bTurnOn)))

(event `self.PlayReactionVFX`
  (params (Reaction :type "ETPP_PongoReactions Enum" :default "None"))
  (`FXSystemComponent.SetIntParameter` (`self.ReactionsVFX`) "FrameToUse" (`BlueprintMapLibrary.Map_Find` (`TPP_PongoReactions.Reaction` (`self.ReactionsDA`)) Reaction))
  (`ActorComponent.Activate` (`self.ReactionsVFX`) true)
  (set `self.bIsPlayingReactionVFX` true))

(fn `UserConstructionScript`
  (`SkinnedMeshComponent.SetLeaderPoseComponent` (`self.FurMesh`) (`self.Mesh`) false false))
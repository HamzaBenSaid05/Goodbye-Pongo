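; Player character Blueprint for Jane, assembled from modular skeletal meshes on the character Mesh.
; The construction script sets Mesh as leader pose component for the SKMJaneJacket and SKMJaneAguayo parts, so both follow its animation.
; On BeginPlay, after the parent logic, it creates a dynamic instance of the body material on one Mesh slot and stores it in MI; nothing here changes its parameters.
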(event `self.ReceiveBeginPlay`
  (`parent.ReceiveBeginPlay`)
  (bind _returnvalue (`PrimitiveComponent.CreateDynamicMaterialInstance` (`self.Mesh`) 2 "/Game/Art/Materials/Characters/Jane/Body/MI_JaneBody.MI_JaneBody" "MI_Body"))
  (set `self.MI` _returnvalue))

(fn `UserConstructionScript`
  (`SkinnedMeshComponent.SetLeaderPoseComponent` (`self.SKM_Jane_Jacket`) (`self.Mesh`) false false)
  (`SkinnedMeshComponent.SetLeaderPoseComponent` (`self.SKM_Jane_Aguayo`) (`self.Mesh`) false false))
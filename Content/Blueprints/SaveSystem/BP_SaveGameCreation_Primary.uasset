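; BP_SaveGameCreation_Primary builds a complete save game from its own variables, covering Pongo, drum and room state.
; CreateCompleteSaveGame wipes SaveSlot0, creates a fresh TPP_SaveGame, fills it through SetUpDrum and SetUpPongo, sets the room index, then saves it back to that slot.
; The setup helpers copy drum ability flags and Pongo's bonding and interaction fields.
; DeleteSaveGame separately clears the same slot.
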(fn `CreateCompleteSaveGame`
  (locals (NewSaveGame :type "TPP_SaveGame Object Reference"))
  (`GameplayStatics.DeleteGameInSlot` "SaveSlot0")
  (bind _returnvalue (`GameplayStatics.CreateSaveGameObject` "/Script/TPP_01.TPP_SaveGame"))
  (set `local.NewSaveGame` _returnvalue)
  (`self.SetUpDrum` (`local.NewSaveGame`))
  (`self.SetUpPongo` (`local.NewSaveGame`))
  ; Room
  (set `TPP_SaveGame.RoomIndex` (`self.RoomIndex`) (`local.NewSaveGame`))
  (`GameplayStatics.SaveGameToSlot` (`local.NewSaveGame`) "SaveSlot0"))

(fn `DeleteSaveGame`
  (`GameplayStatics.DeleteGameInSlot` "SaveSlot0"))

(fn `SetUpDrum`
  (params (SaveGame :type "TPP_SaveGame Object Reference"))
  ; Drum
  (set `TPP_SaveGame.bGoThereActive` (`self.GoThereActive`) (`local.SaveGame`))
  (set `TPP_SaveGame.bInteractActive` (`self.InteractActive`) (`local.SaveGame`))
  (set `TPP_SaveGame.bHasDrum` (`self.HasDrum`) (`local.SaveGame`)))

(fn `SetUpPongo`
  (params (SaveGame :type "TPP_SaveGame Object Reference"))
  ; Pongo
  (set `TPP_SaveGame.BondingValue` (`self.BondingValue`) (`local.SaveGame`))
  (set `TPP_SaveGame.bCanStroll` (`self.CanStroll`) (`local.SaveGame`))
  (set `TPP_SaveGame.bCanBePet` (`self.CanBePet`) (`local.SaveGame`))
  (set `TPP_SaveGame.BondingState` (`self.BondingState`) (`local.SaveGame`)))
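; Drum actor that attaches to a parent component and animates the GoThere command through a marker actor it spawns on BeginPlay.
; While the command runs, its sphere and pylons follow above the marker, with spinning pylons and curve-driven emissive blinking.
; Completion plays a timeline drop with cone scaling, then a return timeline brings the pieces home and resets them.
; Cancellation skips the drop, reusing the return timeline with a swapped finish callback.
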(event `self.ReceiveBeginPlay`
  ;[1 1 1 0.5] Lifecycle
  (bind _returnvalue (`|SpawnActorFromClass` "/Game/Blueprints/Drum/Marker/BP_GoThere_Marker.BP_GoThere_Marker_C" (`KismetMathLibrary.MakeTransform` (0.0 0.0 0.0)) "Undefined" "MultiplyWithRoot" null null))
  (`self.SetMarker` _returnvalue)
  (`NiagaraComponent.SetVariableFloat` (`self.GoThereVFX`) "Speed" 50.0)
  (`NiagaraComponent.SetVariableFloat` (`self.GoThereVFX`) "NumParticles" 8.0)
  (`NiagaraComponent.SetVariableFloat` (`self.GoThereVFX`) "Lifetime" 2.0)
  (set `self.StartingConeScale` (`SceneComponent.RelativeScale3D` (`self.GoThereConeMesh`))))

(event `self.GoThereStarted`
  ;[0.6557 1 0 0.5] GoThere Command
  (`parent.GoThereStarted`)
  (`ActorComponent.SetActive` (`TPP_GoThereMarker.PlayingVFX` (`self.GetMarker`)) false false)
  (`SceneComponent.SetVisibility` (`self.GoThereConeMesh`) true true))

(event `self.GoThere`
  (params (MarkerDirection :type "Vector Structure (by ref)") (StartPositionMarker :type "Vector Structure (by ref)") (DrumHeight :type "Float (single-precision) (by ref)"))
  ;[0.6557 1 0 0.5] GoThere Command
  (if (`self.bGoThereInUse`)
    (`parent.GoThere` MarkerDirection StartPositionMarker DrumHeight)
    (`self.MoveDrumPiecesWithMarker`)))

(event `self.GoThereCompleted`
  (bind (_returnvalue_x _returnvalue_y _returnvalue_z) (`KismetMathLibrary.BreakVector` (`self.K2_GetActorLocation` (`self.GetMarker`))))
  ;[0.6557 1 0 0.5] GoThere Command
  (set `self.bGoThereInUse` false)
  (set `self.MarkerLastPos` (`KismetMathLibrary.MakeVector` _returnvalue_x _returnvalue_y (+ _returnvalue_z (`self.GoThereStartingZOffset`))))
  (`TPP_GoThereMarker.DisableMarker` (`self.GetMarker`))
  (bind (_direction _alpha _scalingalpha) (`Timeline|GoThereCompletedTL` :!via `PlayFromStart`)
    (:`Update`
      (`self.GoThereCompletedDropAnim` _alpha _scalingalpha))
    (:`Finished`
      (`parent.GoThereCompleted`)
      (`SceneComponent.SetVisibility` (`self.GoThereConeMesh`) false true)
      (bind (_direction_2 _alpha_2) (`Timeline|GoThereReturnTL` :!via `PlayFromStart`)
        (:`Update`
          (`self.DropAnim` _alpha_2))
        (:`Finished`
          (`self.ResetGoTherePieces`))))))

(event `self.GoThereCancelled`
  (bind _gotherereturntl (`self.GoThereReturnTL`))
  ;[0.6557 1 0 0.5] GoThere Command
  (`TPP_GoThereMarker.DisableMarker` (`self.GetMarker`))
  (`SceneComponent.SetVisibility` (`self.GoThereConeMesh`) false true)
  (`TimelineComponent.PlayFromStart` _gotherereturntl)
  (`TimelineComponent.SetTimelineFinishedFunc` _gotherereturntl (`|CreateDelegate` :!event `CancelledReturnFinished`)))

(fn `AttachDrum`
  (params (Parent :type "SceneComponent Object Reference"))
  (`self.K2_AttachToComponent` Parent "None" "SnapToTarget" "SnapToTarget" "SnapToTarget")
  (`SceneComponent.K2_AddRelativeLocation` (`self.PlayingVFX`) (0.0 0.0 30.0) false false)
  (`self.SetOwner` (`ActorComponent.GetOwner` (`local.Parent`))))

(fn `CancelledReturnFinished`
  (`self.ResetGoTherePieces`)
  (`parent.GoThereCancelled`)
  (`TimelineComponent.SetTimelineFinishedFunc` :`self` (`self.GoThereReturnTL`)))

(fn `DropAnim`
  (params (Alpha :type "Float (single-precision)"))
  (bind _drumpylons (`self.DrumPylons`))
  (bind _drumsphere (`self.DrumSphere`))
  (`SceneComponent.K2_SetRelativeLocation` _drumsphere (`KismetMathLibrary.VLerp` (`SceneComponent.RelativeLocation` _drumsphere) (0.0 0.0 0.0) (`local.Alpha`)) false false)
  (`SceneComponent.K2_SetRelativeLocation` _drumpylons (`KismetMathLibrary.VLerp` (`SceneComponent.RelativeLocation` _drumpylons) (0.0 0.0 0.0) (`local.Alpha`)) false false))

(fn `GoThereCompletedDropAnim`
  (params (Alpha :type "Float (single-precision)") (ScalingAlpha :type "Float (double-precision)"))
  (locals (TargetPos :type "Vector Structure" :default (0.0 0.0 0.0)))
  (bind (_returnvalue_x _returnvalue_y _returnvalue_z) (`KismetMathLibrary.BreakVector` (`self.K2_GetActorLocation` (`self.GetMarker`))))
  (set `local.TargetPos` (`KismetMathLibrary.VLerp` (`self.MarkerLastPos`) (`KismetMathLibrary.MakeVector` _returnvalue_x _returnvalue_y (- _returnvalue_z (* (`self.GoThereStartingZOffset`) 0.9))) (`local.Alpha`)))
  (`SceneComponent.K2_SetWorldLocation` (`self.DrumSphere`) (`local.TargetPos`) false false)
  (`SceneComponent.K2_SetWorldLocation` (`self.DrumPylons`) (`local.TargetPos`) false false)
  (`SceneComponent.SetRelativeScale3D` (`self.GoThereConeMesh`) (`KismetMathLibrary.VLerp` (`self.StartingConeScale`) (1.0 0.35 0.35) (`local.ScalingAlpha`))))

(fn `MoveDrumPiecesWithMarker`
  (locals (TargetPos :type "Vector Structure" :default (0.0 0.0 0.0)))
  (bind (_returnvalue_x _returnvalue_y _returnvalue_z) (`KismetMathLibrary.BreakVector` (`self.K2_GetActorLocation` (`self.GetMarker`))))
  (set `local.TargetPos` (`KismetMathLibrary.MakeVector` _returnvalue_x _returnvalue_y (+ _returnvalue_z (`self.GoThereStartingZOffset`))))
  (`SceneComponent.K2_SetWorldLocation` (`self.DrumSphere`) (`local.TargetPos`) false false)
  (`SceneComponent.K2_SetWorldLocation` (`self.DrumPylons`) (`local.TargetPos`) false false)
  (`SceneComponent.K2_AddRelativeRotation` (`self.DrumPylons`) (struct :`Yaw` 2.0) false false)
  (bind _output_get (set `self.GoThereElapsedTime` (+ (`self.GoThereElapsedTime`) (`GameplayStatics.GetWorldDeltaSeconds`))))
  (for _array_element (`self.MaterialInstances`)
    (`MaterialInstanceDynamic.SetScalarParameterValue` _array_element "EmissiveBoost" (`KismetMathLibrary.GetRuntimeFloatCurveValue` (`self.BlinkingCurve`) _output_get 1.0))))

(fn `ResetGoTherePieces`
  (`SceneComponent.K2_SetRelativeLocation` (`self.DrumSphere`) (0.0 0.0 0.0) false false)
  (`SceneComponent.K2_SetRelativeLocation` (`self.DrumPylons`) (0.0 0.0 0.0) false false)
  (set `self.GoThereElapsedTime` 0.0)
  (for _array_element (`self.MaterialInstances`)
    (`MaterialInstanceDynamic.SetScalarParameterValue` _array_element "EmissiveBoost" 1.0)
    (`SceneComponent.SetVisibility` (`self.GoThereConeMesh`) false false)
    (`SceneComponent.SetRelativeScale3D` (`self.GoThereConeMesh`) (`self.StartingConeScale`))))

(fn `TogglePylons`
  (params (Param :type Boolean))
  (`FXSystemComponent.SetBoolParameter` (`TPP_GoThereMarker.PylonVFX` (`self.GetMarker`)) "bIsMoving" Param)
  (`FXSystemComponent.SetBoolParameter` (`self.PylonsVFX`) "bIsMoving" Param))

(fn `UserConstructionScript`)
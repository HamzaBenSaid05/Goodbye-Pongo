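; Spawner that manages how the player obtains the drum and persists that in the save game.
; It finds or spawns a hidden BP_Drum and passes it to the character on GameMode's PlayerReady for the acquisition animation.
; If already saved as owned, the drum is granted immediately.
; Otherwise, acquisition enables drum input, removes the mock drum, saves, updates the HUD, and scales the character's orbit object before self-destructing.
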(event `self.ReceiveBeginPlay`
  ;[0 0.08359 0.15 0.5] Binding to GM's PlayerReady Event, spawning drum and binding to its acquisition event
  (bind _astpp_game_mode (cast `TPP_GameMode` (`GameplayStatics.GetGameMode`)))
  (add `TPP_GameMode.OnPlayerReady` _astpp_game_mode (`|CreateDelegate` :!event `PlayerSpawned`))
  (`self.SpawnDrum`))

(event `PlayerSpawned`
  (params (PlayerChar :type "Actor Object Reference"))
  ;[0 0.15 0.0951 0.5] Giving drum ref to the character, needed for the acquisition animation reproduction
  (bind _astpp_player_character (cast `TPP_PlayerCharacter` PlayerChar))
  (`TPP_PlayerCharacter.SetDrum` _astpp_player_character (`self.Drum`))
  ;[0.15 0.05492 0 0.5] In case the char should already have the drum, set it and destroy this
  (bind _astpp_game_instance (cast `TPP_GameInstance` (`GameplayStatics.GetGameInstance`)))
  (if (`TPP_SaveGame.bHasDrum` (`TPP_GameInstance.GetSaveGameObject` _astpp_game_instance))
    (`self.GiveDrumToPlayer` _astpp_player_character)
    (`self.SetActorHiddenInGame` (`self.Drum`) false)
    (`self.K2_DestroyActor`)))

(event `HandleDrumAcquired`
  (params (Char :type "Actor Object Reference"))
  ; This gets called when the acquistion animation finishes, scale the orbit object comp and give the drum to the player
  (bind _astpp_player_character (cast `TPP_PlayerCharacter` Char))
  (`|ExecutionSequence`
    (:`then_0`
      (`KismetSystemLibrary.Delay` 2.5)
      (bind (_direction _alpha) (`Timeline|ScaleCharOrbitComp` :!via `PlayFromStart`)
        (:`Update`
          (bind _drumorbitobject (`TPP_PlayerCharacter.DrumOrbitObject` _astpp_player_character))
          (bind _savedscaleorbitobject (`TPP_PlayerCharacter.SavedScaleOrbitObject` _astpp_player_character))
          (`SceneComponent.SetRelativeScale3D` _drumorbitobject (`KismetMathLibrary.VLerp` (`KismetMathLibrary.Vector_One`) _savedscaleorbitobject _alpha)))
        (:`Finished`
          (`SceneComponent.SetRelativeScale3D` _drumorbitobject _savedscaleorbitobject)
          (`self.K2_DestroyActor`))))
    (:`then_1`
      (`self.GiveDrumToPlayer` _astpp_player_character)
      (bind _astpp_game_instance (cast `TPP_GameInstance` (`GameplayStatics.GetGameInstance`)))
      (bind _returnvalue (`TPP_GameInstance.GetSaveGameObject` _astpp_game_instance))
      (set `TPP_SaveGame.bHasDrum` true _returnvalue)
      (`GameplayStatics.SaveGameToSlot` _returnvalue (`TPP_SaveGame.SaveSlotName` _returnvalue) (`TPP_SaveGame.UserIndex` _returnvalue))
      (bind _asbp_hud_game (cast `/Game/Blueprints/UI/GameHud/BP_HUD_Game` (`PlayerController.GetHUD` (`GameplayStatics.GetPlayerController` 0))))
      (`TPP_HUDGame.ShowDrum` _asbp_hud_game))))

(fn `GiveDrumToPlayer`
  (params (Char :type "Pawn Object Reference"))
  (bind _astpp_player_controller (cast `TPP_PlayerController` (`Pawn.GetController` Char)))
  (`TPP_PlayerController.SetupDrumInput` _astpp_player_controller)
  (bind _returnvalue (`GameplayStatics.GetActorOfClass` "/Game/Blueprints/Drum/BP_MockDrum.BP_MockDrum_C"))
  (`/Engine/EditorBlueprintResources/StandardMacros.IsValid` _returnvalue
    (:`Is Valid`
      (`self.K2_DestroyActor` _returnvalue))))

(fn `SpawnDrum`
  (bind _returnvalue (`GameplayStatics.GetActorOfClass` "/Game/Blueprints/Drum/BP_Drum.BP_Drum_C"))
  (`/Engine/EditorBlueprintResources/StandardMacros.IsValid` _returnvalue
    (:`Is Valid`
      (set `self.Drum` _returnvalue))
    (:`Is Not Valid`
      (bind _returnvalue_2 (`|SpawnActorFromClass` "/Game/Blueprints/Drum/BP_Drum.BP_Drum_C" (`KismetMathLibrary.MakeTransform` (0.0 0.0 0.0)) "Undefined" "MultiplyWithRoot" null null))
      (set `self.Drum` _returnvalue_2)))
  (`self.SetActorHiddenInGame` (`self.Drum`) true)
  (add `TPP_Drum.OnDrumAcquired` (`self.Drum`) (`|CreateDelegate` :!event `HandleDrumAcquired`)))

(fn `UserConstructionScript`)
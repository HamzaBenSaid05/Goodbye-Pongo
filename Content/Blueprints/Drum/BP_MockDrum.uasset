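; BP_MockDrum is the spinning Mock drum, staging the player's drum acquisition sequence and registering itself on Pongo's blackboard.
; It binds to player interaction and camera zoom events.
; MoveToTarget disables input, then Tick walks the player through a middle or final point before a timeline turns them toward the drum and starts the zoom.
; StartAnim plays the acquisition animation; dripping Niagara particle callbacks trigger playing effects and sound.
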(event `self.ReceiveBeginPlay`
  (set `self.TargetLocation` (`SceneComponent.K2_GetComponentLocation` (`self.TargetMiddlePosition`)))
  (`NiagaraComponent.SetVariableActor` (`self.NS_Dripping`) "EventHandler" self)
  (bind _pongoref (`/Game/Blueprints/BP_Statics.GetPongoRef` self))
  (`BlackboardComponent.SetValueAsObject` (`AIBlueprintHelperLibrary.GetBlackboard` (`TPP_Pongo.GetPongoController` _pongoref)) "MockDrum" self)
  (bind _asbp_main_game_mode (cast `/Game/Blueprints/Gameplay/GameModes/BP_MainGameMode` (`GameplayStatics.GetGameMode`)))
  (bind _returnvalue (`TPP_GameMode.GetPlayerCharacterRef` _asbp_main_game_mode))
  (`/Engine/EditorBlueprintResources/StandardMacros.IsValid` _returnvalue
    (:`Is Valid`
      (add `TPP_PlayerCharacter.OnInteractedWithMockDrum` _returnvalue (`|CreateDelegate` :!event `MoveToTarget`))
      (add `TPP_CameraZoomComponent.OnCameraZoom` (`TPP_Camera.CameraZoomComponent` (`self.Camera`)) (`|CreateDelegate` :!event `StartAnim`)))
    (:`Is Not Valid`
      (add `TPP_GameMode.OnPlayerReady` _asbp_main_game_mode (`|CreateDelegate` :!event `OnPlayerReady`))
      (add `TPP_CameraZoomComponent.OnCameraZoom` (`TPP_Camera.CameraZoomComponent` (`self.Camera`)) (`|CreateDelegate` :!event `StartAnim`)))))

(event `OnPlayerReady`
  (params (Player :type "Actor Object Reference"))
  (bind _astpp_player_character (cast `TPP_PlayerCharacter` Player))
  (add `TPP_PlayerCharacter.OnInteractedWithMockDrum` _astpp_player_character (`|CreateDelegate` :!event `MoveToTarget`)))

(event `self.ReceiveParticleData`
  (params (Data :type "Array of BasicParticleData Structure (by ref)") (NiagaraSystem :type "NiagaraSystem Object Reference") (SimulationPositionOffset :type "Vector Structure (by ref)"))
  (bind _emitter_ (`self.Emitter `))
  (`ActorComponent.Activate` (`self.NS_Playing`) true)
  (`TPP_SoundComponent.PlaySound` (`self.SoundComponent`) (struct :`TagName` "Audio.Bongo.Mock") (`SceneComponent.K2_GetComponentLocation` _emitter_) (make `TPP_AudioParameter` 0 "Action") _emitter_)
  (`KismetSystemLibrary.PrintString` "Drumplaying"))

(event `self.ReceiveTick`
  (params (DeltaSeconds :type "Float (single-precision)"))
  (`SceneComponent.K2_AddRelativeRotation` (`self.StaticMesh1`) (`KismetMathLibrary.MakeRotator` 0.0 0.0 (* (`self.RotationSpeed `) (`GameplayStatics.GetWorldDeltaSeconds`))) false false)
  (if (`self.bIsApprochingTargetPoint`)
    (bind _playerref (`/Game/Blueprints/BP_Statics.GetPlayerRef` self))
    (if (> (`KismetMathLibrary.VSize` (- (`self.TargetLocation`) (`self.K2_GetActorLocation` _playerref))) (`self.AprroachDistanceThreshold`))
      (bind _playerref_2 (`/Game/Blueprints/BP_Statics.GetPlayerRef` self))
      (`Pawn.AddMovementInput` _playerref_2 (`KismetMathLibrary.Normal` (- (`self.TargetLocation`) (`self.K2_GetActorLocation` _playerref_2))) 1.5 false)
      (else
        (set `self.TargetLocation` (`SceneComponent.K2_GetComponentLocation` (`self.TargetPlayerPosition`)))
        (if (`KismetMathLibrary.EqualExactly_VectorVector` (`SceneComponent.K2_GetComponentLocation` (`self.TargetPlayerPosition`)) (`self.TargetLocation`))
          (bind _playerref_3 (`/Game/Blueprints/BP_Statics.GetPlayerRef` self))
          (bind (_direction _alpha) (`Timeline|Timeline`)
            (:`Update`
              (bind (_returnvalue_roll _returnvalue_pitch _returnvalue_yaw) (`KismetMathLibrary.BreakRotator` (`self.K2_GetActorRotation` _playerref_3)))
              (bind (_returnvalue_roll_2 _returnvalue_pitch_2 _returnvalue_yaw_2) (`KismetMathLibrary.BreakRotator` (`KismetMathLibrary.FindLookAtRotation` (`self.K2_GetActorLocation` _playerref_3) (`self.K2_GetActorLocation`))))
              (`self.K2_SetActorRotation` _playerref_3 (`KismetMathLibrary.MakeRotator` 0.0 0.0 (`KismetMathLibrary.Lerp` _returnvalue_yaw _returnvalue_yaw_2 _alpha)) false))
            (:`Finished`
              (set `self.bIsApprochingTargetPoint` false)
              (`self.StartZoom`))))))))

(fn `MoveToTarget`
  (bind _returnvalue (`GameplayStatics.GetPlayerController` 0))
  (bind _playerref (`/Game/Blueprints/BP_Statics.GetPlayerRef` self))
  (`/Engine/EditorBlueprintResources/StandardMacros.IsValid` _playerref
    (:`Is Valid`
      (`self.DisableInput` _returnvalue _returnvalue)
      (set `self.bIsApprochingTargetPoint` true)
      (bind _playerref_2 (`/Game/Blueprints/BP_Statics.GetPlayerRef` self))
      (if (> (`KismetMathLibrary.VSize` (- (`self.K2_GetActorLocation` _playerref_2) (`SceneComponent.K2_GetComponentLocation` (`self.TargetPlayerPosition`)))) (`KismetMathLibrary.VSize` (- (`self.K2_GetActorLocation` _playerref_2) (`SceneComponent.K2_GetComponentLocation` (`self.TargetMiddlePosition`)))))
        (set `self.TargetLocation` (`SceneComponent.K2_GetComponentLocation` (`self.TargetMiddlePosition`)))
        (else
          (set `self.TargetLocation` (`SceneComponent.K2_GetComponentLocation` (`self.TargetPlayerPosition`))))))))

(fn `StartAnim`
  (params (State :type "EZoomTrigger Enum" :default "OnZoomInStart"))
  (if (`|EnumEquality` State (`self.StartAnimZoomTrigger`))
    (bind _playerref (`/Game/Blueprints/BP_Statics.GetPlayerRef` self))
    (`TPP_PlayerCharacter.PlayDrumAcquisitionAnimation` _playerref)))

(fn `StartZoom`
  (`TPP_CameraZoomComponent.StartZoom` (`TPP_Camera.CameraZoomComponent` (`self.Camera`)) (`self.In Zoom`) (`self.In Zoom Duration`) (`self.In Zoom Out Duration`) (`self.In Duration Between Transition`) (`self.In Should Wait Before Zoom Out`) (`self.In Zoom in Curve`) (`self.In Zoom Out Curve`)))

(fn `UserConstructionScript`)
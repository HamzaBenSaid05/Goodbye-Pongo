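; BP_UnlockAbility is a pickup trigger that sets either the Go There or Interact ability on the player's Drum, chosen by its Ability variable.
; When the player overlaps its Box, it passes Active to the matching Drum function, shows the drum on the game HUD and destroys itself.
; On BeginPlay it checks the save game and removes itself if Interact is already active; the Go There check does nothing.
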(event `self.ReceiveBeginPlay`
  (bind _returnvalue (`TPP_GameInstance.GetSaveGameObject` (cast `TPP_GameInstance` (`GameplayStatics.GetGameInstance`) :!pure true)))
  (switch `/Game/Blueprints/Drum/E_DrumAbility` (`self.Ability`)
    (:`NewEnumerator0`
      (if (`TPP_SaveGame.bGoThereActive` _returnvalue)
        _))
    (:`NewEnumerator1`
      (if (`TPP_SaveGame.bInteractActive` _returnvalue)
        (`self.K2_DestroyActor`)))))

(event `self.Box.OnComponentBeginOverlap`
  (params (OverlappedComponent :type "PrimitiveComponent Object Reference") (OtherActor :type "Actor Object Reference") (OtherComp :type "PrimitiveComponent Object Reference") (OtherBodyIndex :type Integer) (bFromSweep :type Boolean) (SweepResult :type "HitResult Structure (by ref)"))
  (bind _active (`self.Active`))
  (bind _astpp_player_character (cast `TPP_PlayerCharacter` OtherActor))
  (switch `/Game/Blueprints/Drum/E_DrumAbility` (`self.Ability`)
    (:`NewEnumerator0`
      (bind _drum (`TPP_PlayerCharacter.Drum` _astpp_player_character))
      (`TPP_Drum.EnableGoThere` _drum _active))
    (:`NewEnumerator1`
      (`TPP_Drum.EnableInteract` _drum _active)))
  (bind _asbp_hud_game (cast `/Game/Blueprints/UI/GameHud/BP_HUD_Game` (`PlayerController.GetHUD` (`GameplayStatics.GetPlayerController` 0))))
  (`TPP_HUDGame.ShowDrum` _asbp_hud_game)
  (`self.K2_DestroyActor`))

(fn `UserConstructionScript`)
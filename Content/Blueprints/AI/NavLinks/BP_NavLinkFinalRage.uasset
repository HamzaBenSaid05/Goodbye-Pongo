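; BP_NavLinkFinalRage is an AI nav link that makes the Pongo character play its jump attack when the smart link is reached.
; The SmartLinkReached event fetches the Pongo reference and plays AM_PongoJumpAttack on that character's mesh, without using the event's agent or destination.
; The Blueprint adds no movement or launch logic, and its other events are disabled stubs.
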(event `self.ReceiveSmartLinkReached`
  (params (Agent :type "Actor Object Reference") (Destination :type "Vector Structure (by ref)"))
  (bind _pongoref (`/Game/Blueprints/BP_Statics.GetPongoRef` self))
  (`|PlayMontage` (`Character.Mesh` _pongoref) "/Game/Art/Animations/Characters/Pongo/Retarget/Montages/AM_PongoJumpAttack.AM_PongoJumpAttack"))

(fn `UserConstructionScript`
  (`parent.UserConstructionScript`))
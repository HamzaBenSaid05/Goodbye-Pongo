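; BP_TriggerDestructable is a one-shot overlap trigger that sets off fracturing on a list of destructible actors.
; On collision overlap, it finds each valid actor's BP_DestructableComponentBase and sends the fracture message through BPI_FractureTriggered.
; It then plays a tagged, parameterised TPPSound at its own location and destroys itself.
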(event `self.CollisionComponent.OnComponentBeginOverlap`
  (params (OverlappedComponent :type "PrimitiveComponent Object Reference") (OtherActor :type "Actor Object Reference") (OtherComp :type "PrimitiveComponent Object Reference") (OtherBodyIndex :type Integer) (bFromSweep :type Boolean) (SweepResult :type "HitResult Structure (by ref)"))
  (for _array_element (`self.DestructableToTrigger`)
    (`/Engine/EditorBlueprintResources/StandardMacros.IsValid` _array_element
      (:`Is Valid`
        (bind _returnvalue (`self.GetComponentByClass` _array_element "/Game/Blueprints/Fracture/Component/BP_DestructableComponentBase.BP_DestructableComponentBase_C"))
        (if (`KismetSystemLibrary.IsValid` _returnvalue)
          (if (`KismetSystemLibrary.DoesImplementInterface` _returnvalue "/Game/Blueprints/Fracture/Interface/BPI_FractureTriggered.BPI_FractureTriggered_C")
            (message `/Game/Blueprints/Fracture/Interface/BPI_FractureTriggered.OnFractureTriggered` _returnvalue))))))
  (`TPP_SoundComponent.PlaySound` (`self.TPP_Sound`) (`self.Tag`) (`self.K2_GetActorLocation` self) (make `TPP_AudioParameter` (`self.Parameter Int`) (`self.Parameter Name`)) (`self.RootComponent`))
  (`self.K2_DestroyActor`))

(fn `UserConstructionScript`)
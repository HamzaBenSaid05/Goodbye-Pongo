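; Base component for destructible Chaos Cache Manager actors that plays a cached fracture, then dissolves and destroys the owner.
; BeginPlay caches the owning manager and its Geometry Collection.
; OnFractureTriggered disables collision, triggers the named cache from time zero, optionally shakes the camera and resets any nav modifier to the default area.
; A delayed dissolve creates a dynamic material and enables Tick to interpolate its scalar parameter, then a timer destroys the actor.
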(event `self.ReceiveBeginPlay`
  (bind _aschaos_cache_manager (cast `ChaosCacheManager` (`self.GetOwner`)))
  (set `self.ChasoCacheManagerFracture` _aschaos_cache_manager)
  (bind _output_get (set `self.GeometryCollectionFracture` (`Actor.GetComponentByClass` (`self.GetOwner`) "/Script/GeometryCollectionEngine.GeometryCollectionComponent")))
  (`/Engine/EditorBlueprintResources/StandardMacros.IsValid` _output_get
    (:`Is Valid`
      (`PrimitiveComponent.SetCollisionEnabled` _output_get "QueryAndPhysics"))))

(event `self.OnFractureTriggered`
  (bind _navmodifier (`self.NavModifier`))
  (`ChaosCacheManager.SetCurrentTime` (`self.ChasoCacheManagerFracture`) 0.0)
  (set `ChaosCacheManager.StartTime` 0.0 (`self.ChasoCacheManagerFracture`))
  (`Actor.SetActorEnableCollision` (`self.GetOwner`) false)
  (`ChaosCacheManager.TriggerComponentByCache` (`self.ChasoCacheManagerFracture`) (`self.FractureCacheName`))
  (`KismetSystemLibrary.K2_SetTimerDelegate` (delegate `Dissolve`) (`self.TimeBeforeDissolve`))
  (if (`self.bShouldCameraShake`)
    (`PlayerCameraManager.StartCameraShake` (`GameplayStatics.GetPlayerCameraManager` 0) (`self.Shake Class`) (`self.Scale`) "CameraLocal" (`self.User Play Space Rot`)))
  (`/Engine/EditorBlueprintResources/StandardMacros.IsValid` _navmodifier
    (:`Is Valid`
      (`NavModifierVolume.SetAreaClass` _navmodifier "/Script/NavigationSystem.NavArea_Default"))))

(event `Dissolve`
  (bind _returnvalue (`PrimitiveComponent.CreateDynamicMaterialInstance` (`self.GeometryCollectionFracture`) 0 (`self.Source Material`) "None"))
  (set `self.DynamicMaterialInstance` _returnvalue)
  (`self.SetComponentTickEnabled` true))

(event `self.ReceiveTick`
  (params (DeltaSeconds :type "Float (single-precision)"))
  (bind _dynamicmaterialinstance (`self.DynamicMaterialInstance`))
  (bind _dynamicmaterialinstance_2 (`self.DynamicMaterialInstance`))
  (if (>= (`self.CurrentDissolveValue`) (`self.DissolveValue`))
    (`/Engine/EditorBlueprintResources/StandardMacros.IsValid` _dynamicmaterialinstance
      (:`Is Valid`
        (`MaterialInstanceDynamic.SetScalarParameterValue` _dynamicmaterialinstance (`self.ParameterName`) (`self.DissolveValue`))
        (`KismetSystemLibrary.K2_SetTimerDelegate` (delegate `Destroy`) (`self.TimeBeforeDestroyAfterDissolve`))
        (`self.SetComponentTickEnabled` false)))
    (else
      (bind _output_get (set `self.CurrentDissolveValue` (`KismetMathLibrary.FInterpTo` (`self.CurrentDissolveValue`) (`self.DissolveValue`) DeltaSeconds (`self.InterpSpeedDissolve`))))
      (`/Engine/EditorBlueprintResources/StandardMacros.IsValid` _dynamicmaterialinstance_2
        (:`Is Valid`
          (`MaterialInstanceDynamic.SetScalarParameterValue` _dynamicmaterialinstance_2 (`self.ParameterName`) _output_get))))))

(event `Destroy`
  (`Actor.K2_DestroyActor` (`self.GetOwner`)))
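; Destructible component that persists a door's fractured state across saves, using a DoorTag gameplay tag.
; When fracture triggers, it adds the tag to the save game's UsedDoors container and writes the save slot.
; On BeginPlay with a valid tag, it toggles visibility and collision between the owner and a Chaos cache manager debris actor, so previously destroyed doors appear as debris.
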(event `self.ReceiveBeginPlay`
  (`parent.ReceiveBeginPlay`)
  (set `self.GeometryCollectionDebris` (`Actor.GetComponentByClass` (`self.ChasoCacheManagerDebris`) "/Script/GeometryCollectionEngine.GeometryCollectionComponent"))
  (`self.HandleSave`))

(event `self.OnFractureTriggered`
  (`parent.OnFractureTriggered`)
  (`self.SaveDoor`))

(fn `HandleSave`
  (bind _returnvalue (`self.GetOwner`))
  (bind _returnvalue_2 (`self.GetOwner`))
  (if (`BlueprintGameplayTagLibrary.IsGameplayTagValid` (`self.DoorTag`))
    (if (`BlueprintGameplayTagLibrary.HasTag` (`TPP_SaveGame.UsedDoors` (`/Game/Blueprints/BP_Statics.GetSaveGame` self)) (`self.DoorTag`) true)
      (`Actor.SetActorEnableCollision` _returnvalue false)
      (`Actor.SetActorHiddenInGame` _returnvalue true)
      ;[0.1702 0.2865 0 0.5] Door has been destroyed before, trigger debris simulation
      (`Actor.SetActorHiddenInGame` (`self.ChasoCacheManagerDebris`) false)
      (`Actor.SetActorEnableCollision` (`self.ChasoCacheManagerDebris`) true)
      (else
        (`Actor.SetActorEnableCollision` _returnvalue_2 true)
        (`Actor.SetActorHiddenInGame` _returnvalue_2 false)
        (`Actor.SetActorHiddenInGame` (`self.ChasoCacheManagerDebris`) true)
        (`Actor.SetActorEnableCollision` (`self.ChasoCacheManagerDebris`) false)))))

(fn `SaveDoor`
  (bind _savegameobject (`/Game/Blueprints/BP_Statics.GetSaveGame` self))
  (`BlueprintGameplayTagLibrary.AddGameplayTag` (`TPP_SaveGame.UsedDoors` _savegameobject) (`self.DoorTag`))
  (`GameplayStatics.SaveGameToSlot` _savegameobject (`TPP_SaveGame.SaveSlotName` _savegameobject) (`TPP_SaveGame.UserIndex` _savegameobject)))
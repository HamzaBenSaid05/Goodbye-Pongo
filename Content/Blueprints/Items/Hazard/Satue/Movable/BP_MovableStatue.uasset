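; Movable statue hazard Blueprint that expands or collapses a light cone, with sound for each state.
; ToggleLightCone stops any current audio, then plays a timeline forward or in reverse to scale the cone between zero and its initial size.
; It plays sound at the Emitter through SoundComponent with a StatueState parameter, using a CanPlaySound flag to block repeated expand sounds until the cone collapses.
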(event `self.ToggleLightCone`
  (params (bShouldExpand :type Boolean))
  (bind _emitter (`self.Emitter`))
  (bind _emitter_2 (`self.Emitter`))
  (set `self.Should Expand` bShouldExpand)
  (if (`KismetSystemLibrary.IsValid` (`self.AudioComponent`))
    (`AudioComponent.Stop` (`self.AudioComponent`)))
  (if (`self.Should Expand`)
    (if (`self.CanPlaySound`)
      (set `self.CanPlaySound` false)
      (bind _audiocomp (`TPP_SoundComponent.PlaySound` (`self.SoundComponent`) (`self.Tag`) (`SceneComponent.K2_GetComponentLocation` _emitter_2) (make `TPP_AudioParameter` 0 "StatueState") _emitter_2))
      (set `self.AudioComponent` _audiocomp)
      (bind (_direction _scalingalpha) (`Timeline|Timeline_0` :!label _label)
        (:`Update`
          (`SceneComponent.SetWorldScale3D` (`self.LightCone`) (`KismetMathLibrary.VLerp` (`KismetMathLibrary.Vector_Zero`) (`self.InitialLightConeScale`) _scalingalpha))))
      (else
        (goto _label)))
    (else
      (set `self.CanPlaySound` true)
      (bind _audiocomp_2 (`TPP_SoundComponent.PlaySound` (`self.SoundComponent`) (`self.Tag`) (`SceneComponent.K2_GetComponentLocation` _emitter) (make `TPP_AudioParameter` 1 "StatueState") _emitter))
      (set `self.AudioComponent` _audiocomp_2)
      (goto _label :!via `Reverse`))))

(fn `UserConstructionScript`)
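; A movable statue hazard variant that is replaced by a destructable statue when it finishes moving.
; On the finish-moving event it switches power and reveals the referenced destructable statue actor with its collision disabled.
; It then hides its own hazard mesh and light cone, turns off their collision, and destroys itself.
; Construction defers to the parent class.
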(event `self.OnStatueFinishMoving`
  (bind _destructablestatue (`self.DestructableStatue`))
  (bind _hazardmesh (`self.HazardMesh`))
  (bind _lightcone (`self.LightCone`))
  (`NeedPowerSwitch.SwitchPower`)
  (`self.SetActorHiddenInGame` _destructablestatue false)
  (`self.SetActorEnableCollision` _destructablestatue false)
  (`SceneComponent.SetHiddenInGame` _hazardmesh true true)
  (`PrimitiveComponent.SetCollisionEnabled` _hazardmesh "NoCollision")
  (`SceneComponent.SetHiddenInGame` _lightcone true true)
  (`PrimitiveComponent.SetCollisionEnabled` _lightcone "NoCollision")
  (`self.K2_DestroyActor`))

(fn `UserConstructionScript`
  (`parent.UserConstructionScript`))
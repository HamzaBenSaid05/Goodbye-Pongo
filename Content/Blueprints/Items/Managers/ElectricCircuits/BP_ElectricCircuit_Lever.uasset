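; Electric circuit lever that routes power between two rail sets (A and B), animating the current along their decals.
; A timeline built at runtime from a float curve plays once per segment, driving a dynamic material's Gradient parameter.
; SwitchPower drains the active rails in reverse, swaps sets, then fills the other forward.
; A completed fill calls the parent's SwitchElectricity, except the initial BeginPlay fill.
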(event `self.ReceiveBeginPlay`
  (`self.SetupFillingTL`)
  (`self.SwitchRails` (`self.CurrentRailIsA`))
  (`Timeline|FillingTimeline` :!via `PlayFromStart`))

(event `self.SwitchElectricity`
  (`parent.SwitchElectricity`))

(event `self.SwitchPower`
  (`self.TriggerCircuit`))

(fn `SetupFillingTL`
  (bind _sphere_moving_curve (`self.Sphere Moving Curve`))
  (bind _fillingtimeline (`self.FillingTimeline`))
  (bind (_mintime _maxtime) (`CurveBase.GetTimeRange` _sphere_moving_curve))
  (`TimelineComponent.SetTimelineLength` (`self.FillingTimeline`) (- _maxtime _mintime))
  (`TimelineComponent.AddInterpFloat` (`self.FillingTimeline`) _sphere_moving_curve (`|CreateDelegate` :!event `TLUpdate`) "None" "None")
  (`TimelineComponent.AddEvent` (`self.FillingTimeline`) 0.0 (`|CreateDelegate` :!event `TLStarted`))
  (`TimelineComponent.AddEvent` _fillingtimeline (`TimelineComponent.GetTimelineLength` _fillingtimeline) (`|CreateDelegate` :!event `TLFinished`)))

(fn `SwitchRails`
  (params (UseA :type Boolean))
  (bind _railsinuse (`self.RailsInUse`))
  (bind _output_get (set `self.CurrentRailIsA` UseA))
  (if _output_get
    (`|VariableSetRef` _railsinuse (`self.RailsA`))
    (else
      (`|VariableSetRef` _railsinuse (`self.RailsB`)))))

(fn `TLFinished`
  (if (== (`self.RailIndex`) (`KismetMathLibrary.SelectInt` (`KismetArrayLibrary.Array_LastIndex` (`self.RailsInUse`)) 0 (`self.bGoingForward`)))
    (set `self.RailMaterialInst` null)
    (if (`self.bGoingForward`)
      (if (`self.bIsFirst`)
        (set `self.bIsFirst` false)
        (else
          (`IPowerSwitch.SwitchElectricity`)))
      (else
        (`self.SwitchRails` (not (`self.CurrentRailIsA`)))
        (set `self.bGoingForward` true)
        (set `self.RailIndex` -1)
        (`TimelineComponent.PlayFromStart` (`self.FillingTimeline`))))
    (else
      (set `self.RailMaterialInst` null)
      (`TimelineComponent.PlayFromStart` (`self.FillingTimeline`)))))

(fn `TLStarted`
  (bind _railindex (`self.RailIndex`))
  (if (`self.bGoingForward`)
    (`/Engine/EditorBlueprintResources/StandardMacros.IncrementInt` _railindex
      (:`  `
        _))
    (else
      (`/Engine/EditorBlueprintResources/StandardMacros.DecrementInt` _railindex
        (:`  `
          _))))
  (bind _decal (`DecalActor.Decal` (`|GetArrayItem` (`self.RailsInUse`) (`self.RailIndex`)))
    (:`then`
      (bind _returnvalue (`DecalComponent.CreateDynamicMaterialInstance` _decal))
      (set `self.RailMaterialInst` _returnvalue))
    (:`else`)))

(fn `TLUpdate`
  (params (Value :type "Float (single-precision)"))
  (bind _railmaterialinst (`self.RailMaterialInst`)
    (:`then`
      (`MaterialInstanceDynamic.SetScalarParameterValue` _railmaterialinst "Gradient" (`KismetMathLibrary.SelectFloat` Value (- 1.0 Value) (`self.bGoingForward`))))
    (:`else`)))

(fn `TriggerCircuit`
  (set `self.bGoingForward` false)
  (set `self.RailIndex` (+ (`KismetArrayLibrary.Array_LastIndex` (`self.RailsInUse`)) 1))
  (`TimelineComponent.PlayFromStart` (`self.FillingTimeline`)))

(fn `UserConstructionScript`)
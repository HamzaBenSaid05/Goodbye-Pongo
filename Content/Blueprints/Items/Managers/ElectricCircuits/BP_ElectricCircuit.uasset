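; Electric circuit manager that, once closed, animates its ending rails and powers a door.
; A code-configured timeline, timed from the sphere movement curve, drives a Gradient parameter on each rail decal's dynamic material, replaying rail by rail.
; After the last rail, it switches the door's power, teleports the energy sphere to the end target and leaves the pressure plates pressed with collision disabled.
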(event `self.ReceiveBeginPlay`
  (`parent.ReceiveBeginPlay`)
  (`self.SetupEndingRailsTL`))

(event `self.CloseCircuit`
  (`Timeline|EndingRailsTimeline` :!via `PlayFromStart`))

(fn `EndingRailsTLFinished`
  (if (== (`self.EndingRailsIndex`) (`KismetArrayLibrary.Array_LastIndex` (`self.EndingRails`)))
    (`TPP_BasicItem.SwitchPower` (`self.Door`))
    (`self.K2_SetActorLocation` (`self.EnergySphere`) (`self.K2_GetActorLocation` (`self.EndTarget`)) false false)
    (for _array_element (`self.PressurePlates`)
      (`PrimitiveComponent.SetCollisionEnabled` (`TPP_PressurePlate.CollisionBox` _array_element) "NoCollision")
      (set `TPP_PressurePlate.bIsPlatePressed` true _array_element)
      (`TPP_PressurePlate.PlayAnimation` _array_element)
      (`TPP_CircuitPressurePlate.TogglePlateMeshGraphics` _array_element true)
      (`TPP_CircuitPressurePlate.ToggleSurfacePlateMeshGraphics` _array_element true))
    (else
      (`TimelineComponent.PlayFromStart` (`self.EndingRailsTimeline`)))))

(fn `EndingRailsTLStarted`
  (bind _result (`/Engine/EditorBlueprintResources/StandardMacros.IncrementInt` (`self.EndingRailsIndex`))
    (:`  `
      (bind _decal (`DecalActor.Decal` (`|GetArrayItem` (`self.EndingRails`) _result))
        (:`then`
          (bind _returnvalue (`DecalComponent.CreateDynamicMaterialInstance` _decal))
          (set `self.RailMaterialInst` _returnvalue))
        (:`else`)))))

(fn `EndingRailsTLUpdate`
  (params (Value :type "Float (single-precision)"))
  (bind _railmaterialinst (`self.RailMaterialInst`)
    (:`then`
      (`MaterialInstanceDynamic.SetScalarParameterValue` _railmaterialinst "Gradient" Value))
    (:`else`)))

(fn `SetupEndingRailsTL`
  (bind _endingrailstimeline (`self.EndingRailsTimeline`))
  (bind _endingrailstimeline_2 (`self.EndingRailsTimeline`))
  (bind (_mintime _maxtime) (`CurveBase.GetTimeRange` (`self.SphereMovingCurve`)))
  (`TimelineComponent.SetTimelineLength` _endingrailstimeline (- _maxtime _mintime))
  (`TimelineComponent.AddInterpFloat` _endingrailstimeline "/Game/Blueprints/Items/Managers/ElectricCircuits/C_RailCircuit.C_RailCircuit" (`|CreateDelegate` :!event `EndingRailsTLUpdate`) "None" "None")
  (`TimelineComponent.AddInterpFloat` (`self.EndingRailsTimeline`) "/Game/Blueprints/Items/Managers/ElectricCircuits/C_RailCircuit.C_RailCircuit" (`|CreateDelegate` :!event `EndingRailsTLUpdate`) "None" "None")
  (`TimelineComponent.AddEvent` (`self.EndingRailsTimeline`) 0.0 (`|CreateDelegate` :!event `EndingRailsTLStarted`))
  (`TimelineComponent.AddEvent` _endingrailstimeline_2 (- (`TimelineComponent.GetTimelineLength` _endingrailstimeline_2) (`self.RadiusOffset`)) (`|CreateDelegate` :!event `EndingRailsTLFinished`)))

(fn `UserConstructionScript`)
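; BP_ElectrictSwitch is an interactable electric lever switch that works either as a toggle or as a one-shot.
; On switch, a timeline rotates the lever between its starting and target rotations, then calls the switch-triggered event when finished.
; In toggle mode a FlipFlop alternates playing and reversing the timeline.
; Otherwise the widget is hidden with ticking disabled, and IsAnimating stays true after the pull.
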(event `self.ReceiveBeginPlay`
  (set `self.InitRotation` (`SceneComponent.RelativeRotation` (`self.Lever`))))

(event `self.ImplementationBlueprintSwitch`
  (bind _widgetcomp (`self.WidgetComp`))
  (set `self.bIsAnimating` true)
  (if (`self.bIsToggled`)
    (`/Engine/EditorBlueprintResources/StandardMacros.FlipFlop`
      (:`A`
        (bind (_direction _pulllever) (`Timeline|Timeline` :!label _label)
          (:`Update`
            (`SceneComponent.K2_SetRelativeRotation` (`self.Lever`) (`KismetMathLibrary.RLerp` (`self.InitRotation`) (`self.TargetRotation`) _pulllever) false false))
          (:`Finished`
            (`self.OnElectricSwitchTriggered`)
            (if (`self.bIsToggled`)
              (set `self.bIsAnimating` false)
              (else
                (set `self.bIsAnimating` true))))))
      (:`B`
        (goto _label :!via `Reverse`)))
    (else
      (set `Widget.Visibility` "Hidden" (`WidgetComponent.GetWidget` _widgetcomp))
      (`WidgetComponent.SetTickMode` _widgetcomp "Disabled")
      (goto _label))))

(fn `UserConstructionScript`)
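; BP_CircuitPressurePlateS is a small circuit pressure plate that animates and plays sound as its pressed state changes.
; Its PlayAnimation event reads IsPlatePressed, then plays a timeline forward when pressed or reverses it when released, driving the plate mesh's relative Z location.
; Both directions trigger the small pressure plate sound at the actor's location, with a parameter distinguishing release from press.
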(event `self.PlayAnimation`
  (if (`self.bIsPlatePressed`)
    ; Animation and sound
    (`TPP_SoundComponent.PlaySound` (`self.TPP_Sound`) (struct :`TagName` "Audio.Item.PressurePlate.Small") (`self.K2_GetActorLocation` self) (make `TPP_AudioParameter` 0 "PressurePlateSmall") (`self.RootComponent`))
    (bind (_direction _newtrack_0) (`Timeline|Timeline` :!label _label)
      (:`Update`
        (`SceneComponent.K2_SetRelativeLocation` (`self.PlateMesh`) (`KismetMathLibrary.MakeVector` 0.0 0.0 _newtrack_0) false false)))
    (else
      (`TPP_SoundComponent.PlaySound` (`self.TPP_Sound`) (struct :`TagName` "Audio.Item.PressurePlate.Small") (`self.K2_GetActorLocation` self) (make `TPP_AudioParameter` 1 "PressurePlateSmall") (`self.RootComponent`))
      (goto _label :!via `Reverse`))))

(fn `UserConstructionScript`)
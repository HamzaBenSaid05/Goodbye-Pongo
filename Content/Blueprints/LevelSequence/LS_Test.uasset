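; LS_Test is a level sequence director Blueprint that lets Sequencer drive a cutscene UI widget.
; CheckRefs lazily finds the BP_LevelSequencePlayer actor in the level and caches its LevelSequenceWidget as a WBP_CutSceneWidget, running on creation and before each event.
; The ShowComic and StartAnimation Sequencer events forward their parameters to that widget to display a comic or play a tagged animation.
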(event `self.OnCreated`
  (`self.CheckRefs`))

(event `ShowComic`
  (params (ComicClass :type "/Game/Blueprints/UI/CutScene/WBP_Comic_Base Class Reference"))
  (`self.CheckRefs`)
  (`/Game/Blueprints/UI/CutScene/WBP_CutSceneWidget.ShowComic` (`self.CutSceneWidget`) ComicClass))

(event `StartAnimation`
  (params (Texture :type "Texture2D Soft Object Reference") (StartAtTime :type "Float (single-precision)" :default 0.0) (NumLoopsToPlay :type Integer :default 1) (PlayMode :type "EUMGSequencePlayMode Enum" :default "Forward") (PlaybackSpeed :type "Float (single-precision)" :default 1.0) (AnimationTag :type "GameplayTag Structure"))
  (`self.CheckRefs`)
  (`/Game/Blueprints/UI/CutScene/WBP_CutSceneWidget.StartAnimation` (`self.CutSceneWidget`) Texture StartAtTime NumLoopsToPlay PlayMode PlaybackSpeed AnimationTag))

(fn `CheckRefs`
  (`/Engine/EditorBlueprintResources/StandardMacros.IsValid` (`self.LevelSequencePlayerRef`)
    (:`Is Not Valid`
      (bind _returnvalue (`GameplayStatics.GetActorOfClass` "/Game/Blueprints/LevelSequence/BP_LevelSequencePlayer.BP_LevelSequencePlayer_C"))
      (set `self.LevelSequencePlayerRef` _returnvalue)
      (bind _aswbp_cut_scene_widget (cast `/Game/Blueprints/UI/CutScene/WBP_CutSceneWidget` (`TPP_LevelSequencePlayer.LevelSequenceWidget` (`self.LevelSequencePlayerRef`))))
      (set `self.CutSceneWidget` _aswbp_cut_scene_widget))))
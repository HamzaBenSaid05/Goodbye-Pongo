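; BP_PlayerChangeOST is a directional trigger box that switches the soundtrack when the player character leaves it.
; On end overlap, it dots the player's velocity direction with its own forward vector to choose the forward or backward set of tag, parameter and fade settings.
; It sends that set to the BP_OSTManager found at BeginPlay, and can optionally destroy itself after a forward exit.
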(event `self.ReceiveBeginPlay`
  (bind _returnvalue (`GameplayStatics.GetActorOfClass` "/Game/Blueprints/Sound/BP_OSTManager.BP_OSTManager_C"))
  (set `self.OSTManager` _returnvalue))

(event `self.Box.OnComponentEndOverlap`
  (params (OverlappedComponent :type "PrimitiveComponent Object Reference") (OtherActor :type "Actor Object Reference") (OtherComp :type "PrimitiveComponent Object Reference") (OtherBodyIndex :type Integer))
  (bind _astpp_player_character (cast `TPP_PlayerCharacter` OtherActor))
  (if (> (`KismetMathLibrary.Dot_VectorVector` (`KismetMathLibrary.Normal` (`MovementComponent.Velocity` (`Character.CharacterMovement` _astpp_player_character))) (`self.GetActorForwardVector`)) 0.1)
    (`/Game/Blueprints/Sound/BP_OSTManager.ChangeOST_Event` (`self.OSTManager`) (`self.Forward Tag`) (`self.Forward Parameter Int`) (`self.Forward Parameter Name`) (`self.Forward Time Fade In`) (`self.Forward Time Fade Out`))
    (if (`self.Destroy`)
      (`self.K2_DestroyActor`))
    (else
      (`/Game/Blueprints/Sound/BP_OSTManager.ChangeOST_Event` (`self.OSTManager`) (`self.Backward  Tag`) (`self.Backward  Parameter Int`) (`self.Backward  Parameter Name`) (`self.Backward Time Fade In`) (`self.Backward Time Fade Out`)))))

(fn `UserConstructionScript`)
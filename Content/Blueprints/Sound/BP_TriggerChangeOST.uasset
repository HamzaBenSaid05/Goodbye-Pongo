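; BP_TriggerChangeOST is a trigger volume that changes the game's soundtrack when its Box is overlapped.
; On BeginPlay it finds and caches the level's BP_OSTManager.
; Any Box overlap, with no filter on the other actor, calls the manager's ChangeOSTEvent with the instance's tag, parameter and fade-time variables.
; An optional Destroy flag removes the trigger afterwards, making it one-shot.
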(event `self.ReceiveBeginPlay`
  (bind _returnvalue (`GameplayStatics.GetActorOfClass` "/Game/Blueprints/Sound/BP_OSTManager.BP_OSTManager_C"))
  (set `self.OST Manager` _returnvalue))

(event `self.Box.OnComponentBeginOverlap`
  (params (OverlappedComponent :type "PrimitiveComponent Object Reference") (OtherActor :type "Actor Object Reference") (OtherComp :type "PrimitiveComponent Object Reference") (OtherBodyIndex :type Integer) (bFromSweep :type Boolean) (SweepResult :type "HitResult Structure (by ref)"))
  (`/Game/Blueprints/Sound/BP_OSTManager.ChangeOST_Event` (`self.OST Manager`) (`self.Tag`) (`self.Parameter Int`) (`self.Parameter Name`) (`self.Time Fade In`) (`self.Time Fade Out`))
  (if (`self.Destroy`)
    (`self.K2_DestroyActor`)))

(fn `UserConstructionScript`)
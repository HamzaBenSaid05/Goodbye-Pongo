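; BP_UISoundManager is an actor that plays UI sounds requested through the TPP audio proxy subsystem's UI event.
; Button and checkbox sounds route to SM_UI and stop any playing slider sound.
; Slider sounds use the passed submix and are throttled by a Tick countdown, replaying early only if the previous sound ended or the submix differs.
; Submix routing is written directly onto each played component's Sound asset.
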(event `self.ReceiveBeginPlay`
  (add `TPP_AudioProxySubsystem.OnAudioTableEventUI` (subsystem `TPP_AudioProxySubsystem`) (delegate `PlayUISound`))
  (set `self.Time` (`self.TimerTime`)))

(event `PlayUISound`
  (params (Tag :type "GameplayTag Structure") (Parameter :type "TPP_AudioParameter Structure") (Submix :type "SoundSubmix Object Reference") (Button :type "ButtonType Enum" :default "Button"))
  (bind _audio_slider (`self.Audio Slider`))
  (bind _audio_slider_2 (`self.Audio Slider`))
  (bind _audio_slider_3 (`self.Audio Slider`))
  (set `self.Tag` Tag)
  (set `self.Parameter` Parameter)
  (set `self.Submix` Submix)
  (switch `ButtonType` Button
    (:`Button`
      (bind _audiocomp (`TPP_SoundComponent.PlaySound` (`self.TPP_Sound`) (`self.Tag`) (`self.K2_GetActorLocation` self) (`self.Parameter`) (`self.RootComponent`)))
      (set `SoundBase.SoundSubmixObject` "/Game/Sound/Mixing/SubMixer/SM_UI.SM_UI" (`AudioComponent.Sound` _audiocomp))
      (`/Engine/EditorBlueprintResources/StandardMacros.IsValid` _audio_slider_3
        (:`Is Valid`
          (if (`AudioComponent.IsPlaying` _audio_slider_3)
            (`AudioComponent.Stop` _audio_slider_3)))))
    (:`Slider`
      (`/Engine/EditorBlueprintResources/StandardMacros.IsValid` _audio_slider
        (:`Is Valid`
          (if (`AudioComponent.IsPlaying` _audio_slider)
            (if (`self.ReactiveSound`)
              (bind _audiocomp_2 (`TPP_SoundComponent.PlaySound` (`self.TPP_Sound`) (`self.Tag`) (`self.K2_GetActorLocation` self) (`self.Parameter`) (`self.RootComponent`) :!label _label))
              (bind _output_get (set `self.Audio Slider` _audiocomp_2))
              (set `SoundBase.SoundSubmixObject` (`self.Submix`) (`AudioComponent.Sound` _output_get))
              (set `self.ReactiveSound` false)
              (set `self.Time` (`self.TimerTime`))
              (elif (not (== (`SoundBase.SoundSubmixObject` (`AudioComponent.Sound` (`self.Audio Slider`))) (`self.Submix`)))
                (goto _label)))
            (else
              (goto _label))))
        (:`Is Not Valid`
          (goto _label))))
    (:`CheckBox`
      (bind _audiocomp_3 (`TPP_SoundComponent.PlaySound` (`self.TPP_Sound`) (`self.Tag`) (`self.K2_GetActorLocation` self) (`self.Parameter`) (`self.RootComponent`)))
      (set `SoundBase.SoundSubmixObject` "/Game/Sound/Mixing/SubMixer/SM_UI.SM_UI" (`AudioComponent.Sound` _audiocomp_3))
      (`/Engine/EditorBlueprintResources/StandardMacros.IsValid` _audio_slider_2
        (:`Is Valid`
          (if (`AudioComponent.IsPlaying` _audio_slider_2)
            (`AudioComponent.Stop` _audio_slider_2)))))))

(event `self.ReceiveTick`
  (params (DeltaSeconds :type "Float (single-precision)"))
  (if (`self.ReactiveSound`)
    _
    (elif (<= (`self.Time`) 0.0)
      (set `self.Audio Slider` null)
      (set `self.ReactiveSound` true)
      (else
        (set `self.Time` (- (`self.Time`) DeltaSeconds))))))

(fn `UserConstructionScript`)
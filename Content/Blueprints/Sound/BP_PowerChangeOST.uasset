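; BP_PowerChangeOST is an actor that changes the soundtrack some time after a power switch.
; On BeginPlay it finds and stores the BP_OSTManager in the level.
; SwitchPower starts a timer of configurable length, whose event calls ChangeOSTEvent on the manager with the configured tag, integer parameter and fade-in and fade-out times.
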(event `self.ReceiveBeginPlay`
  (bind _returnvalue (`GameplayStatics.GetActorOfClass` "/Game/Blueprints/Sound/BP_OSTManager.BP_OSTManager_C"))
  (set `self.OSTManager` _returnvalue))

(event `self.SwitchPower`
  (`KismetSystemLibrary.K2_SetTimerDelegate` (delegate `CustomEvent`) (`self.Time`)))

(event `CustomEvent`
  (`/Game/Blueprints/Sound/BP_OSTManager.ChangeOST_Event` (`self.OSTManager`) (`self.Tag`) (`self.Parameter Int`) "None" (`self.Time Fade In`) (`self.Time Fade Out`)))

(fn `UserConstructionScript`)
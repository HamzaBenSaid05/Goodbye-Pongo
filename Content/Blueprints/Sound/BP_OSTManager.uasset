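; BP_OSTManager is the music manager that crossfades soundtrack tracks over a default ambience base started on BeginPlay.
; ChangeOST_Event plays a tagged sound with an integer parameter through TPPSound and stores it in one of two audio component slots.
; Slot choice depends on component validity, and FadeInFadeOut fades the new track in and the other slot out.
; Separate events pause the base layer and the soundtrack slots.
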(event `ChangeOST_Event`
  (params (Tag :type "GameplayTag Structure") (`Parameter Int` :type Integer) (`Parameter Name` :type Name) (TimeFadeIn :type "Float (double-precision)") (TimeFadeOut :type "Float (double-precision)"))
  (set `self.Time Fade In` TimeFadeIn)
  (set `self.Time Fade Out` TimeFadeOut)
  (bind _audiocomp (`TPP_SoundComponent.PlaySound` (`self.TPP_Sound`) Tag (`self.K2_GetActorLocation` self) (make `TPP_AudioParameter` `Parameter Int` `Parameter Name`) (`self.RootComponent`)))
  (set `self.Audio Comp` _audiocomp)
  (`/Engine/EditorBlueprintResources/StandardMacros.IsValid` (`self.FirstAudioComp`)
    (:`Is Valid`
      (`/Engine/EditorBlueprintResources/StandardMacros.IsValid` (`self.SecondAudioComp`)
        (:`Is Valid`
          (set `self.FirstAudioComp` (`self.Audio Comp`))
          (`self.FadeInFadeOut` (`self.FirstAudioComp`) (`self.Time Fade In`) (`self.SecondAudioComp`) (`self.Time Fade Out`)))
        (:`Is Not Valid`
          (set `self.SecondAudioComp` (`self.Audio Comp`))
          (`self.FadeInFadeOut` (`self.SecondAudioComp`) (`self.Time Fade In`) (`self.FirstAudioComp`) (`self.Time Fade Out`)))))
    (:`Is Not Valid`
      (set `self.FirstAudioComp` (`self.Audio Comp`))
      (`self.FadeInFadeOut` (`self.FirstAudioComp`) (`self.Time Fade In`) (`self.SecondAudioComp`) (`self.Time Fade Out`)))))

(event `self.ReceiveBeginPlay`
  (bind _audiocomp (`TPP_SoundComponent.PlaySound` (`self.TPP_Sound`) (struct :`TagName` "Audio.Ambience.Default") (0.0 0.0 0.0) (make `TPP_AudioParameter` 0) (`self.RootComponent`)))
  (set `self.AudioComponentOSTBase` _audiocomp))

(event `PauseBaseOST`
  (params (bPause :type Boolean))
  (`AudioComponent.SetPaused` (`self.AudioComponentOSTBase`) bPause))

(event `PauseOST`
  (params (bPause :type Boolean))
  (bind _secondaudiocomp (`self.SecondAudioComp`))
  (bind _firstaudiocomp (`self.FirstAudioComp`))
  (`/Engine/EditorBlueprintResources/StandardMacros.IsValid` _secondaudiocomp
    (:`Is Valid`
      (`AudioComponent.SetPaused` _secondaudiocomp bPause))
    (:`Is Not Valid`
      _))
  (`/Engine/EditorBlueprintResources/StandardMacros.IsValid` _firstaudiocomp
    (:`Is Valid`
      (`AudioComponent.SetPaused` _firstaudiocomp bPause))))

(fn `FadeInFadeOut`
  (params (FadeInAudioComp :type "AudioComponent Object Reference") (TimeFadeIn :type "Float (double-precision)") (FadeOutAudioComp :type "AudioComponent Object Reference") (TimeFadeOut :type "Float (double-precision)"))
  (`/Engine/EditorBlueprintResources/StandardMacros.IsValid` FadeInAudioComp
    (:`Is Valid`
      (`AudioComponent.FadeIn` FadeInAudioComp TimeFadeIn 1.0 0.0 "Linear")
      (`/Engine/EditorBlueprintResources/StandardMacros.IsValid` FadeOutAudioComp
        (:`Is Valid`
          (`AudioComponent.FadeOut` FadeOutAudioComp TimeFadeOut 0.0 "Linear"))))))

(fn `UserConstructionScript`)
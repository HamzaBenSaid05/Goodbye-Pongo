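; BP_SoundTimer is a trigger volume that plays a tagged sound a set time after an actor with the matching tag overlaps its box.
; The overlap starts a timer, and an in-progress flag ignores further overlaps until it fires.
; The timer event calls TPPSound at the actor's location with an integer parameter and an Emitter source actor.
; It then re-arms if Repeatable, otherwise destroys itself.
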(event `self.Box.OnComponentBeginOverlap`
  (params (OverlappedComponent :type "PrimitiveComponent Object Reference") (OtherActor :type "Actor Object Reference") (OtherComp :type "PrimitiveComponent Object Reference") (OtherBodyIndex :type Integer) (bFromSweep :type Boolean) (SweepResult :type "HitResult Structure (by ref)"))
  (if (`self.ActorHasTag` OtherActor (`self.Tag`))
    (if (not (`self.InProggress`))
      (set `self.InProggress` true)
      (`KismetSystemLibrary.K2_SetTimerDelegate` (delegate `CustomEvent`) (`self.Time`)))))

(event `CustomEvent`
  (`TPP_SoundComponent.PlaySound` (`self.TPP_Sound`) (`self.AudioTag`) (`self.K2_GetActorLocation` self) (make `TPP_AudioParameter` (`self.Paramter Int`) (`self.Parameter Name`)) (`self.Emitter`))
  (if (`self.Repeatable`)
    (set `self.InProggress` false)
    (else
      (`self.K2_DestroyActor`))))

(fn `UserConstructionScript`)
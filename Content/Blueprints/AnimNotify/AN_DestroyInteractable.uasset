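; Anim notify that destroys the AI character's emotional object during an animation and plays an interaction sound.
; It reads the target actor from the owner's AI controller blackboard using a configurable key name.
; If that actor is valid and the owner is a TPP_CharacterBase, it gives the actor a short lifespan for delayed destruction.
; The character's sound component then plays the Pongo interact sound with an Interaction parameter.
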(fn `Received_Notify`
  (params (MeshComp :type "SkeletalMeshComponent Object Reference") (Animation :type "AnimSequenceBase Object Reference") (EventReference :type "AnimNotifyEventReference Structure (by ref)"))
  (returns (ReturnValue :type Boolean))
  (bind _returnvalue (`ActorComponent.GetOwner` MeshComp))
  (bind _asactor (cast `Actor` (`BlackboardComponent.GetValueAsObject` (`AIBlueprintHelperLibrary.GetBlackboard` (`AIBlueprintHelperLibrary.GetAIController` _returnvalue)) (`self.EmotionalObjectKeyName`)) :!pure true))
  (`/Engine/EditorBlueprintResources/StandardMacros.IsValid` _asactor
    (:`Is Valid`
      (bind _astpp_character_base (cast `TPP_CharacterBase` _returnvalue))
      (`Actor.SetLifeSpan` _asactor 1.0)
      (bind _returnvalue_2 (`TPP_CharacterBase.GetSoundComponent` _astpp_character_base))
      (`TPP_SoundComponent.PlaySound` _returnvalue_2 (struct :`TagName` "Audio.Pongo.Interact") (`Actor.K2_GetActorLocation` _astpp_character_base) (make `TPP_AudioParameter` 5 "Interaction") (`Actor.RootComponent` _astpp_character_base))
      (return true))))